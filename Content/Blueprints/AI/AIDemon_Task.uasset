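; Behavior tree task for the demon AI that moves the controlled pawn toward the player's position at a fixed height.
; It reads the player pawn from PSG_GameMode and writes its X/Y with a constant Z to a blackboard vector key.
; An AI MoveTo heads to the same point with zero acceptance radius, finishing on success or aborting on failure, with a debug print either way.
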(event `self.ReceiveExecuteAI`
  (params (OwnerController :type "AIController Object Reference") (ControlledPawn :type "Pawn Object Reference"))
  (bind _aspsg_game_mode (cast `PSG_GameMode` (`GameplayStatics.GetGameMode`)))
  (bind (_x _y) (`KismetMathLibrary.BreakVector3f` (`Actor.K2_GetActorLocation` (`PSG_GameMode.PlayerPawn` _aspsg_game_mode))))
  (bind _returnvalue (`KismetMathLibrary.MakeVector` _x _y 300.0))
  (`BTFunctionLibrary.SetBlackboardValueAsVector` (`self.BBKey`) _returnvalue)
  (bind _movementresult (`|AIMoveTo` ControlledPawn _returnvalue null 0.0)
    (:`OnSuccess`
      (`self.NewFunction_0` "TRUE")
      (`self.FinishExecute` true))
    (:`OnFail`
      (`self.NewFunction_0` (`|GetEnumeratorNameAsString` _movementresult))
      (`self.FinishAbort`))))

(fn `NewFunction_0`
  (params (NewParam :type String))
  (`KismetSystemLibrary.PrintString` NewParam))