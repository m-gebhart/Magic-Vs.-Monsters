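; An interactable double door Blueprint whose two panels slide between their original positions and a shared midpoint.
; The construction script stores each panel's mesh and starting relative location in a struct and calculates the anchor halfway between them.
; Each interaction flips the Open flag and plays or reverses the OpeningAnim timeline, whose alpha lerps both panels from their origins toward that anchor.
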(event `self.OnInteraction`
  (bind ((`originLocation` _originlocation) (`meshComponent` _meshcomponent)) (break `InteractionWorldObject` (`self.rDoor`)))
  (bind ((`originLocation` _originlocation_2) (`meshComponent` _meshcomponent_2)) (break `InteractionWorldObject` (`self.lDoor`)))
  (bind _output_get (set `self.bOpen` (not (`self.bOpen`))))
  (if _output_get
    (bind (_direction _alpha) (`Timeline|OpeningAnim` :!via `PlayFromStart` :!label _label)
      (:`Update`
        (`SceneComponent.K2_SetRelativeLocation` _meshcomponent_2 (`KismetMathLibrary.VLerp` _originlocation_2 (`self.anchorLocation`) _alpha) false false)
        (`SceneComponent.K2_SetRelativeLocation` _meshcomponent (`KismetMathLibrary.VLerp` _originlocation (`self.anchorLocation`) _alpha) false false)))
    (else
      (goto _label :!via `ReverseFromEnd`))))

(fn `FindMidLocation`
  (params (NewParam :type "Vector Structure") (NewParam1 :type "Vector Structure"))
  (returns (NewParam2 :type "Vector Structure"))
  (return (+ NewParam (* (- NewParam1 NewParam) (0.5 0.5 0.5)))))

(fn `UserConstructionScript`
  (bind _leftdoor (`self.LeftDoor`))
  (bind _rightdoor (`self.RightDoor`))
  (bind _relativelocation (`SceneComponent.RelativeLocation` _rightdoor))
  (bind _relativelocation_2 (`SceneComponent.RelativeLocation` _leftdoor))
  (setmembers `InteractionWorldObject` :`StructRef` (`self.lDoor`) :`originLocation` _relativelocation_2 :`meshComponent` _leftdoor)
  (setmembers `InteractionWorldObject` :`StructRef` (`self.rDoor`) :`originLocation` _relativelocation :`meshComponent` _rightdoor)
  (bind _newparam2 (`self.FindMidLocation` _relativelocation_2 _relativelocation))
  (set `self.anchorLocation` _newparam2))